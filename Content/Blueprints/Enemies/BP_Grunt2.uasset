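; BP_Grunt2 is a grunt enemy Blueprint that deals contact damage to the player.
; Both actor overlap and blocking hit events cast the other actor to BP_Player and call Hurt on its Health component with the Damage variable.
; It has no cooldown or other logic of its own, and the construction script only calls the parent's.
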(event EventBeginPlay)

(event Collision|EventActorBeginOverlap
  (params (OtherActor :type Actor%20Object%20Reference))
  (bind _asbp_player (Utilities|Casting|CastToBP_Player OtherActor))
  (Class|Health|Hurt (Variables|/Game/Blueprints/BP_Player.BP_Player_C|GetHealth _asbp_player) (Variables|Default|GetDamage)))

(event EventTick
  (params (DeltaSeconds :type Float%20%28single-precision%29)))

(event Collision|EventHit
  (params (MyComp :type Primitive%20Component%20Object%20Reference) (Other :type Actor%20Object%20Reference) (OtherComp :type Primitive%20Component%20Object%20Reference) (bSelfMoved :type Boolean) (HitLocation :type Vector :default "0, 0, 0") (HitNormal :type Vector :default "0, 0, 0") (NormalImpulse :type Vector :default "0, 0, 0") (Hit :type Hit%20Result%20Structure%20%28by%20ref%29))
  (bind _asbp_player (Utilities|Casting|CastToBP_Player Other))
  (Class|Health|Hurt (Variables|/Game/Blueprints/BP_Player.BP_Player_C|GetHealth _asbp_player) (Variables|Default|GetDamage)))

(fn ConstructionScript
  (|CallParentFunction))