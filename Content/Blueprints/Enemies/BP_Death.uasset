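; BP_Death is a hazard actor that repeatedly damages the player while they overlap it.
; On begin overlap it casts to BP_Player and calls Hurt on the player's Health with its Damage value.
; A one-second Delay loops the hit for as long as a Condition flag is set.
; Any actor ending overlap clears that flag, without a player check, so the loop stops after the pending delay.
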(event EventBeginPlay)

(event Collision|EventActorBeginOverlap
  (params (OtherActor :type Actor%20Object%20Reference))
  (bind _asbp_player (Utilities|Casting|CastToBP_Player OtherActor))
  (Variables|Default|SetCondition true)
  (Class|Health|Hurt (Variables|/Game/Blueprints/BP_Player.BP_Player_C|GetHealth _asbp_player) (Variables|Default|GetDamage) :!label _label)
  (Utilities|FlowControl|Delay 1.0)
  (if (Variables|Default|GetCondition)
    (goto _label)))

(event EventTick
  (params (DeltaSeconds :type Float%20%28single-precision%29)))

(event Collision|EventActorEndOverlap
  (params (OtherActor :type Actor%20Object%20Reference))
  (Variables|Default|SetCondition false))

(fn ConstructionScript
  (|CallParentFunction))