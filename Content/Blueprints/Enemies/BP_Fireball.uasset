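; BP_Fireball is a fireball actor that deals damage on overlap and then destroys itself.
; An overlapped actor qualifies only when the success of a cast to BP_Player equals the Friendly flag.
; A qualifying actor with a valid Health component receives Hurt with the Damage value.
; BeginPlay runs only a Delay with nothing after it, and Tick and construction are empty.
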(event EventBeginPlay
  (Utilities|FlowControl|Delay 1.0))

(event Collision|EventActorBeginOverlap
  (params (OtherActor :type Actor%20Object%20Reference))
  (bind _returnvalue (Actor|GetComponentbyClass OtherActor "/Script/Gauntlet.Health"))
  (if (== (.bSuccess (Utilities|Casting|CastToBP_Player OtherActor)) (Variables|Default|GetFriendly))
    (Utilities|IsValid _returnvalue
      (:Is%20Valid
        (Class|Health|Hurt _returnvalue (Variables|Default|GetDamage))
        (Actor|DestroyActor)))))

(event EventTick
  (params (DeltaSeconds :type Float%20%28single-precision%29)))

(fn ConstructionScript)