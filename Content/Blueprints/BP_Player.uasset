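; Player pawn configured from a character data asset (DA_Elf by default, or the GameInstance's selection) that sets mesh, tint, max speed and max health.
; Enhanced Input drives floating-pawn movement and two yaw aiming modes, heading or incremental, while a cursor-trace look function is left unconnected.
; Holding attack loops a cooldown-length timeline that spawns damage-carrying projectiles.
; Death opens the GameOver level, and debug prints show health and input.
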(event OnDeath(Health)
  (params (Causer :type Actor%20Object%20Reference))
  (Actor|DestroyActor)
  (Game|OpenLevel(byObjectReference) "/Game/Levels/GameOver.GameOver"))

(event Custom|Attack
  (bind _returnvalue (Transformation|GetActorTransform))
  (Game|SpawnActorfromClass (Variables|Default|GetProjectile%20Template) (Math|Transform|MakeTransform (.location _returnvalue) (.rotation _returnvalue) "1.000000,1.000000,1.000000") "Undefined" 0 1e+04 1.0 true (Variables|Default|GetProjectile%20Damage) self))

(event Input|EnhancedActionEvents|EnhancedInputActionIA_Walk
  (params (ActionValue :type Vector%202D%20Structure) (ElapsedSeconds :type Float%20%28double-precision%29) (TriggeredSeconds :type Float%20%28double-precision%29) (InputAction :type Input%20Action%20Object%20Reference :default "/Game/Input/IA_Walk.IA_Walk"))
  (bind _return_value (CallFunction|Vector2DClamp ActionValue 1.0))
  (bind _floatingpawnmovement (Variables|Default|GetFloatingPawnMovement))
  (:Triggered
    (Development|PrintString (Utilities|String|Append "Wal: { X: " "" "; Y: " "" " }"))
    (Class|PawnMovementComponent|AddInputVector _floatingpawnmovement (Math|Vector|MakeVector 0.0 (.x _return_value) 0.0) false)
    (Class|PawnMovementComponent|AddInputVector _floatingpawnmovement (Math|Vector|MakeVector (.y _return_value) 0.0 0.0) false)))

(event Input|EnhancedActionEvents|EnhancedInputActionIA_Look_Using_Normal
  (params (ActionValue :type Vector%202D%20Structure) (ElapsedSeconds :type Float%20%28double-precision%29) (TriggeredSeconds :type Float%20%28double-precision%29) (InputAction :type Input%20Action%20Object%20Reference :default "/Game/Input/IA_Look_Using_Normal.IA_Look_Using_Normal"))
  (bind _returnvalue (Transformation|GetActorLocation))
  (:Triggered
    (Transformation|SetWorldRotation (Variables|Transformation|GetRootComponent) (Math|Rotator|MakeRotator 0.0 0.0 (+ (Math|Trig|RadiansToDegrees (Class|KismetMathLibrary|VectorHeadingAngle (Math|Vector|MakeVector (.x ActionValue) (.y ActionValue) 0.0))) 9e+01)) false false)
    (Rendering|Debug|DrawDebugArrow :LineStart _returnvalue :LineEnd (+ _returnvalue (* 1e+03 (Transformation|GetActorForwardVector))))))

(event Input|EnhancedActionEvents|EnhancedInputActionIA_Attack
  (params (ActionValue :type Boolean) (ElapsedSeconds :type Float%20%28double-precision%29) (TriggeredSeconds :type Float%20%28double-precision%29) (InputAction :type Input%20Action%20Object%20Reference :default "/Game/Input/IA_Attack.IA_Attack"))
  (bind _attack_cooldown (Variables|Default|GetAttack%20Cooldown))
  (:Started
    (Components|Timeline|SetLooping _attack_cooldown true)
    (Timeline|Attack%20Cooldown Play
      (:Finished
        (Components|Timeline|SetNewTime _attack_cooldown 0.0))
      (:Attack
        (CallFunction|Attack)
        (Development|PrintString "Attack"))))
  (:Completed
    (Components|Timeline|SetLooping _attack_cooldown false)))

(event Input|EnhancedActionEvents|EnhancedInputActionIA_Look_Using_Rotation
  (params (ActionValue :type Float%20%28double-precision%29) (ElapsedSeconds :type Float%20%28double-precision%29) (TriggeredSeconds :type Float%20%28double-precision%29) (InputAction :type Input%20Action%20Object%20Reference :default "/Game/Input/IA_Look_Using_Rotation.IA_Look_Using_Rotation"))
  (:Triggered
    (Class|Actor|AddActorWorldRotation (Math|Rotator|MakeRotator 0.0 0.0 ActionValue))))

(event EventBeginPlay
  (bind _returnvalue (Pawn|GetController))
  (bind _return_value (CallFunction|GetGameInstance))
  (bind _asplayer_controller (Utilities|Casting|CastToPlayerController _returnvalue))
  (bind _player_character (Variables|/Game/Blueprints/BP_GameInstance.BP_GameInstance_C|GetPlayer%20Character _return_value))
  (bind _returnvalue_2 (PlayerController|LocalPlayerSubsystems|GetEnhancedInputLocalPlayerSubsystem _asplayer_controller))
  (Utilities|IsValid _player_character
    (:Is%20Valid
      (CallFunction|SetTemplate _player_character)
      (Utilities|IsValid _returnvalue_2
        (:Is%20Valid
          (Input|AddMappingContext _returnvalue_2 "/Game/Input/IMC_GameInput.IMC_GameInput" 0 "(bIgnoreAllPressedKeysUntilRelease=True,bForceImmediately=False)")
          (Components|Timeline|SetTimelineLength (Variables|Default|GetAttack%20Cooldown) (Variables|Default|GetFire%20Cooldown)))))))

(event EventTick
  (params (DeltaSeconds :type Float%20%28single-precision%29))
  (Development|PrintString (Utilities|String|Append "Health" (Utilities|String|ToString(Float) (Variables|/Script/Gauntlet.Health|GetCurrentHealth (Variables|Default|GetHealth)))) true true "(R=1.000000,G=0.000000,B=0.000000,A=1.000000)" 0.0))

(fn ConstructionScript
  (CallFunction|SetTemplate "/Game/Blueprints/CharacterStats/DA_Elf.DA_Elf"))

(fn SetTemplate
  (params (Template :type PDA%20Base%20Character%20Stats%20Object%20Reference))
  (bind _staticmesh (Variables|Default|GetStaticMesh))
  (Utilities|IsValid Template
    (:Is%20Valid
      (Variables|Default|SetCharacter%20Template Template))
    (:Is%20Not%20Valid
      _))
  (Components|StaticMesh|SetStaticMesh _staticmesh (Variables|/Game/Blueprints/CharacterStats/PDA_BaseCharacterStats.PDA_BaseCharacterStats_C|GetMesh (Variables|Default|GetCharacter%20Template)))
  (bind _returnvalue (Rendering|Material|CreateDynamicMaterialInstance "/Game/Materials/M_BaseMaterial.M_BaseMaterial" "None" "None" :!class /Script/Engine.KismetMaterialLibrary))
  (bind _output_get (Variables|Default|SetMaterial _returnvalue))
  (Rendering|Material|SetVectorParameterValue _output_get "Color" (Variables|/Game/Blueprints/CharacterStats/PDA_BaseCharacterStats.PDA_BaseCharacterStats_C|GetColor (Variables|Default|GetCharacter%20Template)) :!class /Script/Engine.MaterialInstanceDynamic)
  (Rendering|Material|SetMaterial _staticmesh 0 _output_get)
  (Variables|/Script/Engine.FloatingPawnMovement|SetMaxSpeed (Variables|Default|GetFloatingPawnMovement) (Variables|/Game/Blueprints/CharacterStats/PDA_BaseCharacterStats.PDA_BaseCharacterStats_C|GetSpeed (Variables|Default|GetCharacter%20Template)))
  (Variables|/Script/Gauntlet.Health|SetMaxHealth (Variables|Default|GetHealth) (Variables|/Game/Blueprints/CharacterStats/PDA_BaseCharacterStats.PDA_BaseCharacterStats_C|GetArmor (Variables|Default|GetCharacter%20Template)))
  (bind _asplayer_controller (Utilities|Casting|CastToPlayerController (Pawn|GetController)))
  (Class|TurnBasedBlueprintLibrary|GetMyPlayerIndex _asplayer_controller))