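; BP_Generator is a destructible enemy spawner that registers with the game instance's generator count.
; BeginPlay resets that count, waits briefly so resets precede increments, then loops forever, spawning a random TemplateEnemies class at its transform on each TimeBetweenSpawn delay.
; When its Health component dies, it decrements the count and destroys itself; Tick prints current health.
; The construction script tints the cube through a dynamic material and sets maximum health.
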(event OnDeath(Health)
  (params (Causer :type Actor%20Object%20Reference))
  (Default|RemoveGenerator (CallFunction|GetGameInstance))
  (Actor|DestroyActor))

(event Custom|Spawn
  (Game|SpawnActorfromClass (.OutItem (Utilities|Array|Random (Variables|Default|GetTemplate%20Enemies))) (Transformation|GetActorTransform) "AlwaysSpawn" 0 15.0 0))

(event EventBeginPlay
  (bind _return_value (CallFunction|GetGameInstance))
  (Variables|/Game/Blueprints/BP_GameInstance.BP_GameInstance_C|SetGenerator%20Count _return_value 0)
  (Utilities|FlowControl|Delay 0.2) ; Not an elegant solution, but enusres generator count is set to zero before incrementing
  (Default|AddGenerator _return_value)
  (Utilities|FlowControl|Sequence :!label _label
    (:then_0
      (CallFunction|Spawn))
    (:then_1
      (Utilities|FlowControl|Delay (Variables|Default|GetTime%20Between%20Spawn))
      (goto _label))))

(event EventTick
  (params (DeltaSeconds :type Float%20%28single-precision%29))
  (Development|PrintString (Utilities|String|ToString(Float) (Variables|/Script/Gauntlet.Health|GetCurrentHealth (Variables|Default|GetHealth))) true true "(R=0.000000,G=0.660000,B=1.000000,A=1.000000)" 0.0))

(fn ConstructionScript
  (bind _returnvalue (Rendering|Material|CreateDynamicMaterialInstance "/Game/Materials/M_BaseMaterial.M_BaseMaterial" "None" "None" :!class /Script/Engine.KismetMaterialLibrary))
  (bind _output_get (Variables|Default|SetMaterial _returnvalue))
  (Rendering|Material|SetVectorParameterValue _output_get "Color" (Variables|Default|GetGenerator%20Color) :!class /Script/Engine.MaterialInstanceDynamic)
  (Rendering|Material|SetMaterial (Variables|Default|GetCube) 0 _output_get)
  (Variables|/Script/Gauntlet.Health|SetMaxHealth (Variables|Default|GetHealth) 2e+01))