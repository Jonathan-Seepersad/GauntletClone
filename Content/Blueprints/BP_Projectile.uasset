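; BP_Projectile is a projectile actor that moves through a ProjectileMovement component and removes itself on timeout or qualifying overlap.
; BeginPlay copies ProjectileSpeed into the component's InitialSpeed, then waits for Lifespan before destroying the actor.
; Overlaps share that destroy step through a Friendly check: friendly projectiles die on non-BP_Player actors, others only on BP_Player.
; It applies no damage itself.
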(event Collision|EventActorBeginOverlap
  (params (OtherActor :type Actor%20Object%20Reference))
  (if (!= (.bSuccess (Utilities|Casting|CastToBP_Player OtherActor)) (Variables|Default|GetFriendly))
    (Actor|DestroyActor)))

(event EventBeginPlay
  (Variables|/Script/Engine.ProjectileMovementComponent|SetInitialSpeed (Variables|Default|GetProjectileMovement) (Variables|Default|GetProjectile%20Speed))
  (Utilities|FlowControl|Delay (Variables|Default|GetLifespan))
  (Actor|DestroyActor))

(fn ConstructionScript)