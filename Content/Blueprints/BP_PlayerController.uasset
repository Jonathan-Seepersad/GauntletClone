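; Player controller that sets up Enhanced Input and a visible mouse cursor for the game.
; On BeginPlay it adds the IMC_GameInput mapping context to the local player subsystem, enables input and shows the cursor.
; The IA_Walk action only prints its X and Y values, with no movement applied.
; The game-only input mode call and the mouse-to-world deprojection are left unconnected.
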(event Input|EnhancedActionEvents|EnhancedInputActionIA_Walk
  (params (ActionValue :type Vector%202D%20Structure) (ElapsedSeconds :type Float%20%28double-precision%29) (TriggeredSeconds :type Float%20%28double-precision%29) (InputAction :type Input%20Action%20Object%20Reference :default "/Game/Input/IA_Walk.IA_Walk"))
  (:Triggered
    (Development|PrintString (Utilities|String|Append "Wal: { X: " (Utilities|String|ToString(Float) (.x ActionValue)) "; Y: " (Utilities|String|ToString(Float) (.y ActionValue)) " }"))))

(event EventBeginPlay
  (bind _self self)
  (bind _returnvalue (PlayerController|LocalPlayerSubsystems|GetEnhancedInputLocalPlayerSubsystem _self))
  (Utilities|IsValid _returnvalue
    (:Is%20Valid
      (Input|AddMappingContext _returnvalue "/Game/Input/IMC_GameInput.IMC_GameInput" 0 "(bIgnoreAllPressedKeysUntilRelease=True,bForceImmediately=False)")
      (Input|EnableInput _self)
      (Variables|Default|SetbShowMouseCursor true))))

(fn ConstructionScript)